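; BP_QuestGiver is a quest-giving actor that shows an interact prompt when the player character enters its trigger radius.
; On Tick, the prompt widget rotates to face the camera.
; Interact toggles a quest menu, creating a new WB_QuestGiver filled from the Quests array each time it opens, and hiding it on close.
; Opening and closing also switch the mouse cursor and input mode.
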(event OnComponentBeginOverlap(TrrigerRadius)
  (params (OverlappedComponent :type Primitive%20Component%20Object%20Reference) (OtherActor :type Actor%20Object%20Reference) (OtherComp :type Primitive%20Component%20Object%20Reference) (OtherBodyIndex :type Integer) (bFromSweep :type Boolean) (SweepResult :type Hit%20Result%20Structure%20%28by%20ref%29))
  (Utilities|Casting|CastToBP_ThirdPersonCharacter OtherActor)
  (Rendering|SetVisibility (Variables|Default|GetInteractWidget) true false))

(event OnComponentEndOverlap(TrrigerRadius)
  (params (OverlappedComponent :type Primitive%20Component%20Object%20Reference) (OtherActor :type Actor%20Object%20Reference) (OtherComp :type Primitive%20Component%20Object%20Reference) (OtherBodyIndex :type Integer))
  (Utilities|Casting|CastToBP_ThirdPersonCharacter OtherActor)
  (Rendering|SetVisibility (Variables|Default|GetInteractWidget) false false))

(event EventInteract
  (bind _returnvalue (Game|GetPlayerController 0))
  (if (not (Variables|Default|GetQuestWBActive))
    (bind _returnvalue_2 (UserInterface|CreateWidget "/Game/Quest_System/WB_QuestGiver.WB_QuestGiver_C"))
    (bind _output_get (Variables|Default|SetQuest%20WB _returnvalue_2))
    (UserInterface|Viewport|AddtoViewport _output_get 0)
    (Variables|Default|SetQuestWBActive true)
    (Variables|/Script/Engine.PlayerController|SetbShowMouseCursor _returnvalue true)
    (Input|SetInputModeGameandUI _returnvalue (Variables|Default|GetQuest%20WB) "DoNotLock" true false)
    (for _array_element (Variables|Default|Getquests)
      (Default|AddQuest (Variables|Default|GetQuest%20WB) _array_element))
    (else
      (Widget|SetVisibility (Variables|Default|GetQuest%20WB) "Hidden")
      (Variables|Default|SetQuestWBActive false)
      (Input|SetInputModeGameOnly (Game|GetPlayerController 0) false)
      (Variables|/Script/Engine.PlayerController|SetbShowMouseCursor (Game|GetPlayerController 0) false))))

(event EventTick
  (params (DeltaSeconds :type Float%20%28single-precision%29))
  (Transformation|SetWorldRotation (Variables|Default|GetInteractWidget) (Math|Rotator|FindLookatRotation (Transformation|GetWorldLocation (Variables|Default|GetInteractWidget)) (Transformation|GetWorldLocation (Variables|/Script/Engine.PlayerCameraManager|GetTransformComponent (Game|GetPlayerCameraManager 0)))) false false))

(fn ConstructionScript)