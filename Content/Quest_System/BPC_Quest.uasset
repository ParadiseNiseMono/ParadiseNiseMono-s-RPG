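; Quest component that shows the active quest on a HUD and tracks its enemy-elimination objectives.
; On BeginPlay it creates the quest HUD, with events to set the quest name and fill the objective list.
; EliminateEnemy removes the enemy from a working target array seeded when empty, writing it back into each open elimination objective by reference.
; An objective completes when that array empties and its ChestToOpen check passes.
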(event Custom|Set%20Active%20Text
  (Rendering|Components|TextRender|SetText (Variables|/Game/Quest_System/WBP_QuestHUD.WBP_QuestHUD_C|GetActiveQuestText (Variables|Default|GetQuest%20HUD)) (Utilities|Text|ToText(String) (.Name (Utilities|Struct|BreakS_Quest (Variables|Default|GetactiveQuest))))))

(event Custom|Set%20Objectives
  (Default|FillObjectives (Variables|Default|GetQuest%20HUD) (.Objectives (Utilities|Struct|BreakS_Quest (Variables|Default|GetactiveQuest)))))

(event Custom|Eliminate%20Enemy
  (params (Enemy%20Eliminated :type Actor%20Object%20Reference))
  (for _array_element (.Objectives (Utilities|Struct|BreakS_Quest (Variables|Default|GetactiveQuest)))
    (if (and (not (.Completed (Utilities|Struct|BreakS_QuestObjective _array_element))) (.IsEliminatedEnemyObjective (Utilities|Struct|BreakS_QuestObjective _array_element)))
      (if (!= (Utilities|Array|Length (Variables|Default|GetActors%20to%20Eliminate%20Array)) 0)
        _
        (else
          (bind _output_get (Variables|Default|SetActors%20to%20Eliminate%20Array (.ActorsToEliminate (Utilities|Struct|BreakS_QuestObjective _array_element))))))
      (Utilities|Array|RemoveItem _output_get Enemy%20Eliminated)
      (|SetBy-RefVar _array_element (Utilities|Struct|MakeS_QuestObjective (.NameAim (Utilities|Struct|BreakS_QuestObjective _array_element)) false (Variables|Default|GetActors%20to%20Eliminate%20Array) (.ChestToOpen (Utilities|Struct|BreakS_QuestObjective _array_element)) (.IsEliminatedEnemyObjective (Utilities|Struct|BreakS_QuestObjective _array_element)) (.IsChestObjective (Utilities|Struct|BreakS_QuestObjective _array_element))))
      (Development|PrintString (Utilities|String|ToString(Integer) (Utilities|Array|Length (Variables|Default|GetActors%20to%20Eliminate%20Array))))
      (if (and (== (Utilities|Array|Length (Variables|Default|GetActors%20to%20Eliminate%20Array)) 0) (== (.ChestToOpen (Utilities|Struct|BreakS_QuestObjective _array_element)) 0))
        (Default|CompleteObjective (Variables|Default|GetQuest%20HUD) _array_element)
        (|SetBy-RefVar _array_element (Utilities|Struct|MakeS_QuestObjective (.NameAim (Utilities|Struct|BreakS_QuestObjective _array_element)) true 0 (.ChestToOpen (Utilities|Struct|BreakS_QuestObjective _array_element)) (.IsEliminatedEnemyObjective (Utilities|Struct|BreakS_QuestObjective _array_element)) (.IsChestObjective (Utilities|Struct|BreakS_QuestObjective _array_element))))))))

(event EventBeginPlay
  (bind _returnvalue (UserInterface|CreateWidget "/Game/Quest_System/WBP_QuestHUD.WBP_QuestHUD_C"))
  (bind _output_get (Variables|Default|SetQuest%20HUD _returnvalue))
  (UserInterface|Viewport|AddtoViewport _output_get 0))