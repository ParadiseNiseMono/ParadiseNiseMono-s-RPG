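; Player combat component for BP_ThirdPersonCharacter, handling a four-step melee combo and bow aiming.
; Attack input briefly turns the character toward control rotation and plays montages by AttackIndex, buffering presses made mid-attack for SwordAttackCombo to continue.
; A looping-timer blade trace and a one-shot sphere trace damage "Damageable" actors with camera shake, sound and blood.
; Bow input switches rotation mode and toggles a crosshair widget; Q unequips the bow.
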(event Custom|Sword%20Attack
  ;[0.05127 0.05127 0.05127] Combo System
  ;;[0.05127 0.05127 0.05127] Sword Attack
  (if (Variables|Default|GetisAttacking)
    (Variables|Default|Setsave%20Sttack? true)
    (else
      (Variables|Default|SetisAttacking true)
      (switch int (Variables|Default|GetAttack%20Index)
        (:0
          (CallFunction|Attack1)
          (Variables|Default|SetCan%20Attack? true))
        (:1
          (CallFunction|Attack2)
          (Variables|Default|SetCan%20Attack? true))
        (:2
          (CallFunction|Attack3)
          (Variables|Default|SetCan%20Attack? true))
        (:3
          (CallFunction|Attack4)
          (Variables|Default|SetCan%20Attack? true))))))

(event Custom|SwordAttackCombo
  ;[0.05127 0.05127 0.05127] Combo System
  ;;[0.05127 0.05127 0.05127] Combo Continue
  (if (Variables|Default|Getsave%20Sttack?)
    (Variables|Default|Setsave%20Sttack? false)
    (switch int (Variables|Default|GetAttack%20Index)
      (:0
        (CallFunction|Attack1)
        (Variables|Default|SetCan%20Attack? true))
      (:1
        (CallFunction|Attack2)
        (Variables|Default|SetCan%20Attack? true))
      (:2
        (CallFunction|Attack3)
        (Variables|Default|SetCan%20Attack? true))
      (:3
        (CallFunction|Attack4)
        (Variables|Default|SetCan%20Attack? true)))))

(event Custom|Start%20Sword%20Trace
  ;[0.05127 0.05127 0.05127] Sword Trace
  (bind _returnvalue (Utilities|Time|SetTimerbyEvent (delegate Custom|Sword%20Trace%20Loop) 0.001 true))
  (Variables|Default|SetSwordTraceLoop _returnvalue))

(event Custom|Sword%20Trace%20Loop
  ;[0.05127 0.05127 0.05127] Sword Trace
  (bind (_outhit _returnvalue) (Collision|SphereTraceByChannel (Transformation|GetWorldLocation (Variables|/Game/ThirdPerson/Blueprints/BP_ThirdPersonCharacter.BP_ThirdPersonCharacter_C|GetSword%20Top%20Poing (Variables|Default|GetCharacterBP))) (Transformation|GetWorldLocation (Variables|/Game/ThirdPerson/Blueprints/BP_ThirdPersonCharacter.BP_ThirdPersonCharacter_C|GetSword%20Bottom (Variables|Default|GetCharacterBP))) 12.0 "TraceTypeQuery1" false 0 "None" true "(R=1.000000,G=0.000000,B=0.000000,A=1.000000)" "(R=0.000000,G=1.000000,B=0.000000,A=1.000000)" 0.3))
  (if _returnvalue
    (if (Actor|ActorHasTag (.HitActor (Collision|BreakHitResult _outhit)) "Damageable")
      (Utilities|FlowControl|DoOnce false :!label _label
        (:Completed
          (Game|Damage|ApplyDamage (.HitActor (Collision|BreakHitResult _outhit)) 1e+01 0 0)
          (Camera|PlayWorldCameraShake "/Game/Blueprints/BP_SwordHitCameraShake.BP_SwordHitCameraShake_C" (.Location (Collision|BreakHitResult _outhit)) 0.0 2e+03)
          (CallFunction|PlaySwordSounds)
          (Effects|SpawnEmitteratLocation "/Game/FXs/Particles/Blood/P_Blood_Splat_Cone.P_Blood_Splat_Cone" (.Location (Collision|BreakHitResult _outhit)) (Math|Rotator|MakeRotfromXY (.Normal (Collision|BreakHitResult _outhit)) (.Normal (Collision|BreakHitResult _outhit))) "0.400000,0.400000,0.400000" true "AutoRelease")
          (Utilities|FlowControl|Delay 0.4)
          (goto _label Reset))))))

(event Custom|Stop%20Sword%20Trace
  ;[0.05127 0.05127 0.05127] Sword Trace
  (Utilities|Time|ClearandInvalidateTimerbyHandle (Variables|Default|GetSwordTraceLoop)))

(event Custom|Sphere%20Trace
  (bind _characterbp (Variables|Default|GetCharacterBP))
  (bind _sphere_trace (Variables|/Game/ThirdPerson/Blueprints/BP_ThirdPersonCharacter.BP_ThirdPersonCharacter_C|GetSphere%20Trace _characterbp))
  (bind _returnvalue (Transformation|GetWorldLocation _sphere_trace))
  ;[0.15 0.15 0.15 0.5] Shpere Trace(For Stab And Kick)
  (bind (_outhit _returnvalue_2) (Collision|SphereTraceByChannel _returnvalue _returnvalue 25.0 "TraceTypeQuery1" false 0 "None"))
  (if _returnvalue_2
    (if (Actor|ActorHasTag (.HitActor (Collision|BreakHitResult _outhit)) "Damageable")
      (Game|Damage|ApplyDamage (.HitActor (Collision|BreakHitResult _outhit)) 1e+01 0 0)
      (Camera|PlayWorldCameraShake "/Game/Blueprints/BP_SwordHitCameraShake.BP_SwordHitCameraShake_C" (.Location (Collision|BreakHitResult _outhit)) 0.0 2e+03)
      (CallFunction|PlaySwordSounds)
      (Effects|SpawnEmitteratLocation "/Game/FXs/Particles/Blood/P_Blood_Splat_Cone.P_Blood_Splat_Cone" (.Location (Collision|BreakHitResult _outhit)) (Math|Rotator|MakeRotfromXY (.Normal (Collision|BreakHitResult _outhit)) (.Normal (Collision|BreakHitResult _outhit))) "0.400000,0.400000,0.400000" true "AutoRelease"))))

(event Custom|PlaySwordSounds
  ;[0.05127 0.05127 0.05127] PlaySwordHitSounds
  (Audio|PlaySoundatLocation "/Game/Audio/SwordHits/MS_Sword.MS_Sword" (Transformation|GetActorLocation (Components|GetOwner)) "0, 0, 0" 1.0 1.0 0.0 "/Game/Audio/SA_Character.SA_Character" 0 0 0))

(event Custom|Stop%20Combo
  ;[0.05127 0.05127 0.05127] Combo System
  ;;[0.05127 0.05127 0.05127] Stop Combo/Attack
  (Variables|Default|SetisAttacking false)
  (Variables|Default|SetAttack%20Index 0))

(event Custom|Attack4
  ;[0.05127 0.05127 0.05127] Combo System
  ;;[0.05127 0.05127 0.05127] Attack4
  (Utilities|FlowControl|DoOnce false :!label _label
    (:Completed
      (Utilities|FlowControl|Delay 0.1)
      (Animation|Montage|PlayMontage (Variables|Default|GetCharacterMesh) "/Game/Characters/RPG_Character/Animetions/SwordAttacks/Attack3_Montage.Attack3_Montage"
        (:then
          (Variables|Default|SetAttack%20Index 4)
          (goto _label Reset))
        (:OnCompleted
          (Variables|Default|SetCan%20Attack? true))
        (:OnInterrupted
          (CallFunction|StopCombo))))))

(event Custom|Attack1
  ;[0.05127 0.05127 0.05127] Combo System
  ;;[0.05127 0.05127 0.05127] Attack1
  (Utilities|FlowControl|DoOnce false :!label _label
    (:Completed
      (Utilities|FlowControl|Delay 0.1)
      (Animation|Montage|PlayMontage (Variables|Default|GetCharacterMesh) "/Game/Characters/RPG_Character/Animetions/SwordAttacks/Attack1_Montage.Attack1_Montage"
        (:then
          (Variables|Default|SetAttack%20Index 1)
          (goto _label Reset))
        (:OnCompleted
          (Variables|Default|SetCan%20Attack? true))
        (:OnInterrupted
          (CallFunction|StopCombo))))))

(event Custom|Attack2
  ;[0.05127 0.05127 0.05127] Combo System
  ;;[0.05127 0.05127 0.05127] Attack2
  (Utilities|FlowControl|DoOnce false :!label _label
    (:Completed
      (Utilities|FlowControl|Delay 0.1)
      (Animation|Montage|PlayMontage (Variables|Default|GetCharacterMesh) "/Game/Characters/RPG_Character/Animetions/SwordAttacks/Attack2_Montage.Attack2_Montage"
        (:then
          (Variables|Default|SetAttack%20Index 2)
          (goto _label Reset))
        (:OnCompleted
          (Variables|Default|SetCan%20Attack? true))
        (:OnInterrupted
          (CallFunction|StopCombo))))))

(event Custom|Attack3
  ;[0.05127 0.05127 0.05127] Combo System
  ;;[0.05127 0.05127 0.05127] Attack3
  (Utilities|FlowControl|DoOnce false :!label _label
    (:Completed
      (Utilities|FlowControl|Delay 0.1)
      (Animation|Montage|PlayMontage (Variables|Default|GetCharacterMesh) "/Game/Characters/RPG_Character/Animetions/SwordAttacks/Kick_Montage.Kick_Montage"
        (:then
          (Variables|Default|SetAttack%20Index 3)
          (goto _label Reset))
        (:OnCompleted
          (Variables|Default|SetCan%20Attack? true))
        (:OnInterrupted
          (CallFunction|StopCombo))))))

(event Input|EnhancedActionEvents|EnhancedInputActionIA_Attack
  (params (ActionValue :type Boolean) (ElapsedSeconds :type Float%20%28double-precision%29) (TriggeredSeconds :type Float%20%28double-precision%29) (InputAction :type Input%20Action%20Object%20Reference :default "/Game/ThirdPerson/Input/Actions/IA_Attack.IA_Attack"))
  ;[0.05127 0.05127 0.05127] Combo System
  ;;[0.05127 0.05127 0.05127] Attack Input
  (:Started
    (if (Variables|Default|GetCan%20Attack?)
      (CallFunction|SwordAttack)
      (Variables|Default|SetOrient%20Attack true)
      (Utilities|FlowControl|Delay 0.3)
      (Variables|Default|SetOrient%20Attack false))))

(event Input|EnhancedActionEvents|EnhancedInputActionIA_BowShoot
  (params (ActionValue :type Boolean) (ElapsedSeconds :type Float%20%28double-precision%29) (TriggeredSeconds :type Float%20%28double-precision%29) (InputAction :type Input%20Action%20Object%20Reference :default "/Game/ThirdPerson/Input/Actions/IA_BowShoot.IA_BowShoot"))
  (bind _characterbp (Variables|Default|GetCharacterBP))
  (bind _characterbp_2 (Variables|Default|GetCharacterBP))
  (bind _charactermovement (Variables|/Script/Engine.Character|GetCharacterMovement _characterbp))
  (bind _charactermovement_2 (Variables|/Script/Engine.Character|GetCharacterMovement _characterbp_2))
  (:Started
    (if (Variables|Default|Gethas%20Bow)
      (Variables|Default|SetCan%20Attack? false)
      (Variables|Default|Setaiming%20Bow true)
      (Default|EquipBowinHand _characterbp_2)
      (Variables|/Script/Engine.CharacterMovementComponent|SetbUseControllerDesiredRotation _charactermovement_2 true)
      (Variables|/Script/Engine.CharacterMovementComponent|SetbOrientRotationToMovement _charactermovement_2 false)
      (bind _returnvalue (UserInterface|CreateWidget "/Game/UI/WBP_Bow_Crosshair.WBP_Bow_Crosshair_C"))
      (bind _output_get (Variables|Default|SetBow%20Crosshair%20WBP _returnvalue))
      (UserInterface|Viewport|AddtoViewport _output_get 0)))
  (:Completed
    (if (Variables|Default|Gethas%20Bow)
      (Variables|Default|SetCan%20Attack? false)
      (Variables|Default|Setaiming%20Bow false)
      (Variables|/Script/Engine.CharacterMovementComponent|SetbUseControllerDesiredRotation _charactermovement false)
      (Variables|/Script/Engine.CharacterMovementComponent|SetbOrientRotationToMovement _charactermovement true)
      (Utilities|FlowControl|Delay 0.2)
      (bind _bow_crosshair_wbp (Variables|Default|GetBow%20Crosshair%20WBP)
        (:then
          (Widget|RemovefromParent _bow_crosshair_wbp)
          (Variables|Default|SetBow%20Crosshair%20WBP 0))
        (:else)))))

(event EventBeginPlay
  (bind _asbp_third_person_character (Utilities|Casting|CastToBP_ThirdPersonCharacter (Components|GetOwner)))
  (Variables|Default|SetCharacterBP _asbp_third_person_character)
  (Variables|Default|SetCharacterMesh (Variables|/Script/Engine.Character|GetMesh _asbp_third_person_character)))

(event EventTick
  (params (DeltaSeconds :type Float%20%28single-precision%29))
  (bind _characterbp (Variables|Default|GetCharacterBP))
  (bind _returnvalue (Transformation|GetActorRotation _characterbp))
  (bind (_roll _pitch) (Math|Rotator|BreakRotator _returnvalue))
  (if (Variables|Default|GetOrient%20Attack)
    (Transformation|SetActorRotation _characterbp (Math|Rotator|MakeRotator _roll _pitch (.yaw (Math|Interpolation|RInterpTo _returnvalue (Pawn|GetControlRotation _characterbp :!class /Script/Engine.Pawn) DeltaSeconds 1e+01))))))

(event Input|KeyboardEvents|Q
  (params (Key :type Key%20Structure :default "None"))
  (:Pressed
    (if (Variables|Default|Gethas%20Bow)
      (Default|UnequipBowinHand (Variables|Default|GetCharacterBP)))))