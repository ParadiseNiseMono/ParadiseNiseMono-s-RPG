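; Player stats component for BP_ThirdPersonCharacter that tracks health, stamina, XP and level.
; On BeginPlay it caches the owning character after a one-tick delay, then its functions change stats and push values straight to that character's HUD widget.
; Decrease functions return whether the stat is depleted, and reaching max XP triggers a level-up that resets XP, raises the threshold and plays sounds.
; IncreaseMaxHealth derives the new maximum from MaxStamina, not MaxHealth.
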(event EventBeginPlay
  (Utilities|FlowControl|DelayUntilNextTick)
  (bind _asbp_third_person_character (Utilities|Casting|CastToBP_ThirdPersonCharacter (Components|GetOwner)))
  (Variables|Default|SetPlayer%20Character%20BP _asbp_third_person_character)
  (Progress|SetPercent (Variables|/Game/UI/WBP_HUD.WBP_HUD_C|GetStamina (Variables|/Game/ThirdPerson/Blueprints/BP_ThirdPersonCharacter.BP_ThirdPersonCharacter_C|GetHUD%20Widget (Variables|Default|GetPlayer%20Character%20BP))) (/ (Variables|Stamina|GetCurrent%20Stamina) (Variables|Stamina|GetMax%20Stamina)))
  (Progress|SetPercent (Variables|/Game/UI/WBP_HUD.WBP_HUD_C|GetHealth (Variables|/Game/ThirdPerson/Blueprints/BP_ThirdPersonCharacter.BP_ThirdPersonCharacter_C|GetHUD%20Widget (Variables|Default|GetPlayer%20Character%20BP))) (/ (Variables|Health|GetCurrent%20Health) (Variables|Health|GetMax%20Health)))
  (Rendering|Components|TextRender|SetText (Variables|/Game/UI/WBP_HUD.WBP_HUD_C|GetHealthText (Variables|/Game/ThirdPerson/Blueprints/BP_ThirdPersonCharacter.BP_ThirdPersonCharacter_C|GetHUD%20Widget (Variables|Default|GetPlayer%20Character%20BP))) (Utilities|Text|ToText(Float) (Variables|Health|GetCurrent%20Health) "HalfToEven"))
  (Progress|SetPercent (Variables|/Game/UI/WBP_HUD.WBP_HUD_C|GetXPBar (Variables|/Game/ThirdPerson/Blueprints/BP_ThirdPersonCharacter.BP_ThirdPersonCharacter_C|GetHUD%20Widget (Variables|Default|GetPlayer%20Character%20BP))) (/ (Variables|XP|GetXP) (Variables|XP|GetMaxXP)))
  (Rendering|Components|TextRender|SetText (Variables|/Game/UI/WBP_HUD.WBP_HUD_C|GetXPText (Variables|/Game/ThirdPerson/Blueprints/BP_ThirdPersonCharacter.BP_ThirdPersonCharacter_C|GetHUD%20Widget (Variables|Default|GetPlayer%20Character%20BP))) (Utilities|Text|FormatText "{Current XP}/{Max XP}" (Variables|XP|GetXP) (Variables|XP|GetMaxXP)))
  (Rendering|Components|TextRender|SetText (Variables|/Game/UI/WBP_HUD.WBP_HUD_C|GetLevelText (Variables|/Game/ThirdPerson/Blueprints/BP_ThirdPersonCharacter.BP_ThirdPersonCharacter_C|GetHUD%20Widget (Variables|Default|GetPlayer%20Character%20BP))) (Utilities|Text|ToText(Integer) (Variables|XP|GetLevel))))

(event EventTick
  (params (DeltaSeconds :type Float%20%28single-precision%29)))

(fn DecreaseHealth
  (params (Damage :type Float%20%28double-precision%29))
  (bind _player_character_bp (Variables|Default|GetPlayer%20Character%20BP))
  (bind _hud_widget (Variables|/Game/ThirdPerson/Blueprints/BP_ThirdPersonCharacter.BP_ThirdPersonCharacter_C|GetHUD%20Widget _player_character_bp))
  (if (not (<= (Variables|Health|GetCurrent%20Health) 0.0))
    (bind _output_get (Variables|Health|SetCurrent%20Health (- (Variables|Health|GetCurrent%20Health) Damage)))
    (Progress|SetPercent (Variables|/Game/UI/WBP_HUD.WBP_HUD_C|GetHealth _hud_widget) (/ _output_get (Variables|Health|GetMax%20Health)))
    (Rendering|Components|TextRender|SetText (Variables|/Game/UI/WBP_HUD.WBP_HUD_C|GetHealthText _hud_widget) (Utilities|Text|ToText(Float) (Variables|Health|GetCurrent%20Health) "HalfToEven"))
    (if (<= (Variables|Health|GetCurrent%20Health) 0.0)
      _
      (else
        (return false))))
  (return true))

(fn IncreaseMaxHealth
  (params (Heal%20Count :type Float%20%28double-precision%29))
  (bind _player_character_bp (Variables|Default|GetPlayer%20Character%20BP))
  (bind _hud_widget (Variables|/Game/ThirdPerson/Blueprints/BP_ThirdPersonCharacter.BP_ThirdPersonCharacter_C|GetHUD%20Widget _player_character_bp))
  (bind _output_get (Variables|Health|SetMax%20Health (+ (Variables|Stamina|GetMax%20Stamina) Heal%20Count)))
  (Progress|SetPercent (Variables|/Game/UI/WBP_HUD.WBP_HUD_C|GetHealth _hud_widget) _output_get)
  (Rendering|Components|TextRender|SetText (Variables|/Game/UI/WBP_HUD.WBP_HUD_C|GetHealthText _hud_widget) (Utilities|Text|ToText(Float) (Variables|Health|GetCurrent%20Health) "HalfToEven")))

(fn DecreaseStamina
  (params (Stamina%20Decreasement :type Float%20%28double-precision%29))
  (if (not (<= (Variables|Stamina|GetCurrent%20Stamina) 0.0))
    (bind _output_get (Variables|Stamina|SetCurrent%20Stamina (- (Variables|Stamina|GetCurrent%20Stamina) Stamina%20Decreasement)))
    (Progress|SetPercent (Variables|/Game/UI/WBP_HUD.WBP_HUD_C|GetStamina (Variables|/Game/ThirdPerson/Blueprints/BP_ThirdPersonCharacter.BP_ThirdPersonCharacter_C|GetHUD%20Widget (Variables|Default|GetPlayer%20Character%20BP))) (/ _output_get (Variables|Stamina|GetMax%20Stamina)))
    (if (<= (Variables|Stamina|GetCurrent%20Stamina) 0.0)
      _
      (else
        (return false))))
  (return true))

(fn IncreaseMaxStamina
  (params (Added%20Stamina :type Float%20%28double-precision%29))
  (Variables|Stamina|SetMax%20Stamina (+ (Variables|Stamina|GetMax%20Stamina) Added%20Stamina))
  (Progress|SetPercent (Variables|/Game/UI/WBP_HUD.WBP_HUD_C|GetStamina (Variables|/Game/ThirdPerson/Blueprints/BP_ThirdPersonCharacter.BP_ThirdPersonCharacter_C|GetHUD%20Widget (Variables|Default|GetPlayer%20Character%20BP))) (/ (Variables|Stamina|GetCurrent%20Stamina) (Variables|Stamina|GetMax%20Stamina))))

(fn IncreaseHealth
  (params (Added%20Health :type Float%20%28double-precision%29))
  (bind _player_character_bp (Variables|Default|GetPlayer%20Character%20BP))
  (bind _hud_widget (Variables|/Game/ThirdPerson/Blueprints/BP_ThirdPersonCharacter.BP_ThirdPersonCharacter_C|GetHUD%20Widget _player_character_bp))
  (Variables|Health|SetCurrent%20Health (+ (Variables|Health|GetCurrent%20Health) Added%20Health))
  (if (> (Variables|Health|GetCurrent%20Health) (Variables|Health|GetMax%20Health))
    (Variables|Health|SetCurrent%20Health (Variables|Health|GetMax%20Health)))
  (Progress|SetPercent (Variables|/Game/UI/WBP_HUD.WBP_HUD_C|GetHealth _hud_widget) (/ (Variables|Health|GetCurrent%20Health) (Variables|Health|GetMax%20Health)))
  (Rendering|Components|TextRender|SetText (Variables|/Game/UI/WBP_HUD.WBP_HUD_C|GetHealthText _hud_widget) (Utilities|Text|ToText(Float) (Variables|Health|GetCurrent%20Health) "HalfToEven")))

(fn IncreaseStamina
  (params (Added%20Stamina :type Float%20%28double-precision%29))
  (Variables|Stamina|SetCurrent%20Stamina (+ (Variables|Stamina|GetCurrent%20Stamina) Added%20Stamina))
  (if (> (Variables|Stamina|GetCurrent%20Stamina) (Variables|Stamina|GetMax%20Stamina))
    (bind _output_get (Variables|Stamina|SetCurrent%20Stamina (Variables|Stamina|GetMax%20Stamina)))
    (bind _player_character_bp (Variables|Default|GetPlayer%20Character%20BP)
      (:then
        (bind _hud_widget (Variables|/Game/ThirdPerson/Blueprints/BP_ThirdPersonCharacter.BP_ThirdPersonCharacter_C|GetHUD%20Widget _player_character_bp)
          (:then
            _)
          (:else)))
      (:else)))
  (Progress|SetPercent (Variables|/Game/UI/WBP_HUD.WBP_HUD_C|GetStamina _hud_widget) (/ _output_get (Variables|Stamina|GetMax%20Stamina))))

(fn IncreaseXP
  (params (Added%20XP :type Float%20%28double-precision%29))
  (Variables|XP|SetXP (+ Added%20XP (Variables|XP|GetXP)))
  (if (>= (Variables|XP|GetXP) (Variables|XP|GetMaxXP))
    (LevelandXP|IncreaseLevel 1))
  (Progress|SetPercent (Variables|/Game/UI/WBP_HUD.WBP_HUD_C|GetXPBar (Variables|/Game/ThirdPerson/Blueprints/BP_ThirdPersonCharacter.BP_ThirdPersonCharacter_C|GetHUD%20Widget (Variables|Default|GetPlayer%20Character%20BP))) (/ (Variables|XP|GetXP) (Variables|XP|GetMaxXP)))
  (Rendering|Components|TextRender|SetText (Variables|/Game/UI/WBP_HUD.WBP_HUD_C|GetXPText (Variables|/Game/ThirdPerson/Blueprints/BP_ThirdPersonCharacter.BP_ThirdPersonCharacter_C|GetHUD%20Widget (Variables|Default|GetPlayer%20Character%20BP))) (Utilities|Text|FormatText "{Current XP}/{Max XP}" (Variables|XP|GetXP) (Variables|XP|GetMaxXP))))

(fn IncreaseLevel
  (params (Added%20Level :type Integer))
  (Variables|XP|SetLevel (+ Added%20Level (Variables|XP|GetLevel)))
  (Variables|XP|SetMaxXP (+ (Variables|XP|GetMaxXP) 1e+02))
  (Variables|XP|SetXP 0.0)
  (Rendering|Components|TextRender|SetText (Variables|/Game/UI/WBP_HUD.WBP_HUD_C|GetLevelText (Variables|/Game/ThirdPerson/Blueprints/BP_ThirdPersonCharacter.BP_ThirdPersonCharacter_C|GetHUD%20Widget (Variables|Default|GetPlayer%20Character%20BP))) (Utilities|Text|ToText(Integer) (Variables|XP|GetLevel)))
  (Audio|PlaySound2D "/Game/Audio/UI/epiclevelup.epiclevelup" 1.0 1.0 0.0 0 0)
  (Audio|PlaySound2D "/Game/Audio/UI/levelup.levelup" 1.0 1.0 0.0 0 0))