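; BP_AI is an enemy character that can attack, take hits and be stealth-assassinated from behind.
; An overlap radius toggles an assassinate prompt, which turns toward the camera along with the health bar.
; Damage plays a random hit montage and launches it along the player's forward vector; BPCPlayerStates decides death, triggering ragdoll.
; StealthBackAssassin plays the paired victim montage, returns an alignment location and rotation, and starts delayed death and destruction.
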(event OnComponentBeginOverlap(AssassinRadius)
  (params (OverlappedComponent :type Primitive%20Component%20Object%20Reference) (OtherActor :type Actor%20Object%20Reference) (OtherComp :type Primitive%20Component%20Object%20Reference) (OtherBodyIndex :type Integer) (bFromSweep :type Boolean) (SweepResult :type Hit%20Result%20Structure%20%28by%20ref%29))
  (Utilities|Casting|CastToBP_ThirdPersonCharacter OtherActor)
  (Rendering|SetVisibility (Variables|Default|GetAssassinateWidget) true false))

(event OnComponentEndOverlap(AssassinRadius)
  (params (OverlappedComponent :type Primitive%20Component%20Object%20Reference) (OtherActor :type Actor%20Object%20Reference) (OtherComp :type Primitive%20Component%20Object%20Reference) (OtherBodyIndex :type Integer))
  (Utilities|Casting|CastToBP_ThirdPersonCharacter OtherActor)
  (Rendering|SetVisibility (Variables|Default|GetAssassinateWidget) false false))

(event Custom|Ragdoll
  ;[0.15 0.15 0.15 0.5] Ragdoll
  (Utilities|FlowControl|Sequence
    (:then_0
      (Utilities|FlowControl|Delay 1.75)
      (Audio|PlaySoundatLocation "/Game/Audio/Grunts-Hit/SC_Death.SC_Death" (Transformation|GetActorLocation) "0, 0, 0" 1.0 1.0 0.0 0 0 0 0))
    (:then_1
      (Utilities|FlowControl|Delay 2.5)
      (Physics|SetSimulatePhysics (Variables|Character|GetMesh) true)
      (Actor|DestroyActor))))

(event Collision|EventActorBeginOverlap
  (params (OtherActor :type Actor%20Object%20Reference)))

(event EventTick
  (params (DeltaSeconds :type Float%20%28single-precision%29))
  (Transformation|SetWorldRotation (Variables|Default|GetAssassinateWidget) (Math|Rotator|FindLookatRotation (Transformation|GetWorldLocation (Variables|Default|GetAssassinateWidget)) (Transformation|GetWorldLocation (Variables|/Script/Engine.PlayerCameraManager|GetTransformComponent (Game|GetPlayerCameraManager 0)))) false false))

(event Game|Damage|EventAnyDamage
  (params (Damage :type Float%20%28single-precision%29) (DamageType :type Damage%20Type%20Object%20Reference) (InstigatedBy :type Controller%20Object%20Reference) (DamageCauser :type Actor%20Object%20Reference))
  (Animation|PlayAnimMontage (Utilities|Array|Get(acopy) (Variables|Default|GetHItAnims) (Math|Random|RandomIntegerinRange 0 (- (Utilities|Array|Length (Variables|Default|GetHItAnims)) 1))) 1.0 "None")
  (bind _asbp_third_person_character (Utilities|Casting|CastToBP_ThirdPersonCharacter (Game|GetPlayerCharacter 0)))
  (Character|LaunchCharacter (* (Math|Vector|GetForwardVector (Transformation|GetActorRotation _asbp_third_person_character)) 7e+02) false false)
  (Audio|PlaySoundatLocation "/Game/Audio/Grunts-Hit/death1.death1" (Transformation|GetActorLocation) "0, 0, 0" 1.0 (Math|Random|RandomFloatinRange 0.5 1.0) 0.0 "/Game/Audio/SA_Character.SA_Character" 0 0 0)
  (bind _isplayerdead (Default|DecreaseHealth (Variables|Default|GetBPC_PlayerStates) Damage))
  (if _isplayerdead
    (Physics|SetSimulatePhysics (Variables|Character|GetMesh) true)
    (Audio|PlaySoundatLocation "/Game/Audio/Grunts-Hit/SC_Death.SC_Death" (Transformation|GetActorLocation) "0, 0, 0" 1.0 1.0 0.0 0 0 0 0)
    (Rendering|SetVisibility (Variables|Default|GetHealth%20Bar%20WBP) false false)
    (Collision|SetCollisionEnabled (Variables|Collision|GetCapsuleComponent) "NoCollision")))

(event EventBeginPlay
  (bind _aswbp_dummy_health_bar (Utilities|Casting|CastToWBP_DummyHealthBar (UserInterface|GetWidget (Variables|Default|GetHealth%20Bar%20WBP))))
  (Variables|Default|SetWBP%20Dummy%20Health%20Bar _aswbp_dummy_health_bar))

(fn ConstructionScript)

(fn Attack
  (bind _returnvalue (Animation|PlayAnimMontage "/Game/Characters/RPG_Character/Animetions/SwordAttacks/Attack1_Montage.Attack1_Montage" 1.0 "None"))
  (return _returnvalue))

(fn StealthBackAssassin
  (Animation|PlayAnimMontage "/Game/Characters/RPG_Character/Animetions/Assassinations/Paired_Knife_Stealth_KidneyAndNeck_Vic_Montage.Paired_Knife_Stealth_KidneyAndNeck_Vic_Montage" 1.0 "None")
  (CallFunction|Ragdoll)
  (Rendering|SetVisibility (Variables|Default|GetAssassinateWidget) false false)
  (Collision|SetCollisionEnabled (Variables|Collision|GetCapsuleComponent) "NoCollision")
  (return (Transformation|GetWorldLocation (Variables|Default|GetAssasin%20REF)) (Transformation|GetActorRotation)))